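; Shooting range penalty target that subtracts points from the player's BP_FPShooter character when shot.
; BeginPlay caches the character, and overlaps from BP_FirstPersonProjectile on the Head and Body components deduct points, with a larger penalty for the head.
; Timeline logic for sliding the mesh back and forth toward End at TargetSpeed exists but is never triggered, and the saved start location is unused.
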(event `self.ReceiveBeginPlay`
  (bind (_returnvalue_x _returnvalue_y _returnvalue_z) (`KismetMathLibrary.BreakVector` (`self.K2_GetActorLocation`)))
  (set `self.Start` (`KismetMathLibrary.MakeVector` _returnvalue_x _returnvalue_y _returnvalue_z))
  (bind _asbp_fpshooter (cast `/Game/Variant_Shooter/Blueprints/FirstPerson/BP_FPShooter` (`GameplayStatics.GetPlayerCharacter` 0)))
  (set `self.character ref` _asbp_fpshooter))

(event `self.Head.OnComponentBeginOverlap`
  (params (OverlappedComponent :type "PrimitiveComponent Object Reference") (OtherActor :type "Actor Object Reference") (OtherComp :type "PrimitiveComponent Object Reference") (OtherBodyIndex :type Integer) (bFromSweep :type Boolean) (SweepResult :type "HitResult Structure (by ref)"))
  (bind _character_ref (`self.character ref`))
  (cast `/Game/Variant_Shooter/Blueprints/Pickups/Projectiles/BP_FirstPersonProjectile` OtherActor)
  (set `/Game/Variant_Shooter/Blueprints/FirstPerson/BP_FPShooter.Points` (- (`/Game/Variant_Shooter/Blueprints/FirstPerson/BP_FPShooter.Points` _character_ref) 10) _character_ref))

(event `self.Body.OnComponentBeginOverlap`
  (params (OverlappedComponent :type "PrimitiveComponent Object Reference") (OtherActor :type "Actor Object Reference") (OtherComp :type "PrimitiveComponent Object Reference") (OtherBodyIndex :type Integer) (bFromSweep :type Boolean) (SweepResult :type "HitResult Structure (by ref)"))
  (bind _character_ref (`self.character ref`))
  (cast `/Game/Variant_Shooter/Blueprints/Pickups/Projectiles/BP_FirstPersonProjectile` OtherActor)
  (set `/Game/Variant_Shooter/Blueprints/FirstPerson/BP_FPShooter.Points` (- (`/Game/Variant_Shooter/Blueprints/FirstPerson/BP_FPShooter.Points` _character_ref) 5) _character_ref))

(fn `UserConstructionScript`)