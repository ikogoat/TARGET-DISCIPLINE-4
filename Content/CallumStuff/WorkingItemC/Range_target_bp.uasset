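; Shooting range target that slides back and forth and awards the player points when hit.
; On BeginPlay it caches the first-person character and loops two timelines, lerping between its start location and a fixed world Y coordinate.
; Head and Body overlaps that pass a cast (class unresolved) add points to the character, more for the head, then destroy the overlapping actor.
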(event `self.ReceiveBeginPlay`
  (bind (_returnvalue_x _returnvalue_y _returnvalue_z) (`KismetMathLibrary.BreakVector` (`self.K2_GetActorLocation`)))
  (set `self.Start` (`KismetMathLibrary.MakeVector` _returnvalue_x _returnvalue_y _returnvalue_z))
  (set `self.End` (`KismetMathLibrary.MakeVector` _returnvalue_x -920.0 _returnvalue_z))
  (bind _asbp_first_person_character (cast `/Game/FirstPerson/Blueprints/BP_FirstPersonCharacter` (`GameplayStatics.GetPlayerCharacter` 0)))
  (set `self.character ref` _asbp_first_person_character)
  (bind (_direction _move) (`Timeline|Move` :!via `PlayFromStart` :!label _label)
    (:`Update`
      (`self.K2_SetActorLocation` (`KismetMathLibrary.VLerp` (`self.Start`) (`self.End`) _move)))
    (:`Finished`
      (bind (_direction_2 _move_2) (`Timeline|Move Back` :!via `ReverseFromEnd`)
        (:`Update`
          (`self.K2_SetActorLocation` (`KismetMathLibrary.VLerp` (`self.Start`) (`self.End`) _move_2)))
        (:`Finished`
          (goto _label :!via `PlayFromStart`))))))

(event `self.Head.OnComponentBeginOverlap`
  (params (OverlappedComponent :type "PrimitiveComponent Object Reference") (OtherActor :type "Actor Object Reference") (OtherComp :type "PrimitiveComponent Object Reference") (OtherBodyIndex :type Integer) (bFromSweep :type Boolean) (SweepResult :type "HitResult Structure (by ref)"))
  (bind _character_ref (`self.character ref`))
  (bind _asbp_first_person_projectile (cast `` OtherActor))
  (set `/Game/FirstPerson/Blueprints/BP_FirstPersonCharacter.points` (+ (`/Game/FirstPerson/Blueprints/BP_FirstPersonCharacter.points` _character_ref) 10) _character_ref)
  (`self.K2_DestroyActor` _asbp_first_person_projectile))

(event `self.Body.OnComponentBeginOverlap`
  (params (OverlappedComponent :type "PrimitiveComponent Object Reference") (OtherActor :type "Actor Object Reference") (OtherComp :type "PrimitiveComponent Object Reference") (OtherBodyIndex :type Integer) (bFromSweep :type Boolean) (SweepResult :type "HitResult Structure (by ref)"))
  (bind _character_ref (`self.character ref`))
  (bind _asbp_first_person_projectile (cast `` OtherActor))
  (set `/Game/FirstPerson/Blueprints/BP_FirstPersonCharacter.points` (+ (`/Game/FirstPerson/Blueprints/BP_FirstPersonCharacter.points` _character_ref) 5) _character_ref)
  (`self.K2_DestroyActor` _asbp_first_person_projectile))

(fn `UserConstructionScript`)